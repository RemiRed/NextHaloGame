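; First-person character controller Blueprint with movement, mouse look, a camera-direction dash, double jump and wall running.
; Jumps launch through a DoN that resets on landing or wall-detector overlap.
; On "RunWall" surfaces while airborne, a timeline with Space held removes gravity, constrains movement horizontally and pushes along the entry view direction, while side detectors drive timelines rolling the view.
; Dash briefly launches, stops movement, then recharges only once HasKilled is true.
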(event `InputAxis|Horizontal`
  (params (AxisValue :type "Float (single-precision)"))
  (bind (_returnvalue_roll _returnvalue_pitch _returnvalue_yaw) (`KismetMathLibrary.BreakRotator` (`self.GetControlRotation`)))
  ;[1 1 1] Player Movement
  (if (not (`self.OnWall`))
    (`self.AddMovementInput` (`KismetMathLibrary.GetRightVector` (`KismetMathLibrary.MakeRotator` 0.0 0.0 _returnvalue_yaw)) AxisValue)))

(event `InputAxis|Vertical`
  (params (AxisValue :type "Float (single-precision)"))
  (bind (_returnvalue_roll _returnvalue_pitch _returnvalue_yaw) (`KismetMathLibrary.BreakRotator` (`self.GetControlRotation`)))
  ;[1 1 1] Player Movement
  (if (not (`self.OnWall`))
    (`self.AddMovementInput` (`KismetMathLibrary.GetForwardVector` (`KismetMathLibrary.MakeRotator` 0.0 0.0 _returnvalue_yaw)) AxisValue)))

(event `self.ReceiveBeginPlay`
  ;[1 1 1] Enable
  (`MovementComponent.SetPlaneConstraintEnabled` (`self.CharacterMovement`) true))

(event `InputAxis|MouseLookHorizontal`
  (params (AxisValue :type "Float (single-precision)"))
  ;[1 1 1] MouseInput
  (`self.AddControllerYawInput` AxisValue))

(event `InputAxis|MouseLookVertical`
  (params (AxisValue :type "Float (single-precision)"))
  ;[1 1 1] MouseInput
  (`self.AddControllerPitchInput` AxisValue))

(event `InputAction|Dash`
  (params (Key :type "Key Structure"))
  ;[1 1 1] Dash
  (:`Pressed`
    (if (`self.Can dash`)
      (`self.LaunchCharacter` (* (`SceneComponent.GetForwardVector` (`self.Camera`)) 7000.0))
      (`KismetSystemLibrary.Delay` 0.15)
      (set `self.Can dash` false)
      (`MovementComponent.StopMovementImmediately` (`self.CharacterMovement`) :!label _label)
      (`KismetSystemLibrary.Delay` 1.0)
      (if (`self.HasKilled`)
        (set `self.Can dash` true)
        (else
          (set `self.Can dash` false)
          (goto _label))))))

(event `self.OnLanded`
  (params (Hit :type "HitResult Structure (by ref)"))
  (goto _label_2 :!via `Reset`))

(event `InputAction|Jump`
  (params (Key :type "Key Structure"))
  (:`Pressed`
    ;[1 1 1] DoubleJump
    (bind _counter (`/Engine/EditorBlueprintResources/StandardMacros.Do N` 2 :!label _label_2)
      (:`Exit`
        (switch `int` _counter
          (:`1`
            _)
          (:`2`
            _))
        (bind _returnvalue (`PrimitiveComponent.GetPhysicsLinearVelocity` (`self.CapsuleComponent`) "None"))
        (`self.LaunchCharacter` (`KismetMathLibrary.MakeVector` 0.0 0.0 (+ (* (.z _returnvalue) -1.0) (`self.jumpForce`)))))))
  (:`Released`
    (`self.StopJumping`)))

(event `self.RightDetector.OnComponentEndOverlap`
  (params (OverlappedComponent :type "PrimitiveComponent Object Reference") (OtherActor :type "Actor Object Reference") (OtherComp :type "PrimitiveComponent Object Reference") (OtherBodyIndex :type Integer))
  (bind _returnvalue (`self.K2_GetActorRotation`))
  ;[1 1 1] WallRunningSmoothing
  (if (and (`self.ActorHasTag` (stale `self.RightDetector.OnComponentBeginOverlap` OtherActor) "RunWall") (`NavMovementComponent.IsFalling` (`self.CharacterMovement`)))
    (bind (_direction _newtrack_0) (`Timeline|SmoothRotRight` :!via `ReverseFromEnd` :!label _label_3)
      (:`Update`
        (`Controller.SetControlRotation` (`GameplayStatics.GetPlayerController` 0) (`KismetMathLibrary.RLerp` _returnvalue (`KismetMathLibrary.MakeRotator` -20.0 (.pitch _returnvalue) (.yaw _returnvalue)) _newtrack_0))))))

(event `self.WallDetection.OnComponentBeginOverlap`
  (params (OverlappedComponent :type "PrimitiveComponent Object Reference") (OtherActor :type "Actor Object Reference") (OtherComp :type "PrimitiveComponent Object Reference") (OtherBodyIndex :type Integer) (bFromSweep :type Boolean) (SweepResult :type "HitResult Structure (by ref)"))
  (bind _charactermovement (`self.CharacterMovement`))
  (bind _charactermovement_2 (`self.CharacterMovement`))
  ;[1 1 1] WallRun
  (`|ExecutionSequence`
    (:`then_0`
      (goto _label_2 :!via `Reset`))
    (:`then_1`
      (set `self.PlayerDirr` (`SceneComponent.GetForwardVector` (`self.Camera`)))
      (if (and (`self.ActorHasTag` OtherActor "RunWall") (`NavMovementComponent.IsFalling` (`self.CharacterMovement`)))
        (set `self.OnWall` true)
        (`Timeline|WallRun` :!label _label_4
          (:`Update`
            (if (> (`PlayerController.GetInputKeyTimeDown` (`GameplayStatics.GetPlayerController` 0) "SpaceBar") 0.0)
              (if (`self.OnWall`)
                (set `CharacterMovementComponent.GravityScale` 0.0 _charactermovement)
                (`MovementComponent.SetPlaneConstraintNormal` _charactermovement (0.0 0.0 1.0))
                (`CharacterMovementComponent.AddForce` _charactermovement (* (`self.PlayerDirr`) 30000.0))
                (else
                  (set `CharacterMovementComponent.GravityScale` 1.0 _charactermovement_2 :!label _label_5)
                  (`MovementComponent.SetPlaneConstraintNormal` _charactermovement_2 (0.0 0.0 0.0))
                  (set `self.OnWall` false)))
              (else
                (goto _label_5)))))))))

(event `self.RightDetector.OnComponentBeginOverlap`
  (params (OverlappedComponent :type "PrimitiveComponent Object Reference") (OtherActor :type "Actor Object Reference") (OtherComp :type "PrimitiveComponent Object Reference") (OtherBodyIndex :type Integer) (bFromSweep :type Boolean) (SweepResult :type "HitResult Structure (by ref)"))
  ;[1 1 1] WallRunningSmoothing
  (if (and (`self.ActorHasTag` OtherActor "RunWall") (`NavMovementComponent.IsFalling` (`self.CharacterMovement`)))
    (goto _label_3 :!via `PlayFromStart`)))

(event `self.WallDetection.OnComponentEndOverlap`
  (params (OverlappedComponent :type "PrimitiveComponent Object Reference") (OtherActor :type "Actor Object Reference") (OtherComp :type "PrimitiveComponent Object Reference") (OtherBodyIndex :type Integer))
  ;[1 1 1] WallRun
  (`|ExecutionSequence`
    (:`then_0`
      (goto _label_4 :!via `Stop`))
    (:`then_1`
      (if (`self.ActorHasTag` OtherActor "RunWall")
        (goto _label_5)))))

(event `self.LeftDetector.OnComponentBeginOverlap`
  (params (OverlappedComponent :type "PrimitiveComponent Object Reference") (OtherActor :type "Actor Object Reference") (OtherComp :type "PrimitiveComponent Object Reference") (OtherBodyIndex :type Integer) (bFromSweep :type Boolean) (SweepResult :type "HitResult Structure (by ref)"))
  (bind _returnvalue (`self.K2_GetActorRotation`))
  ;[1 1 1] WallRunningSmoothing
  (if (and (`NavMovementComponent.IsFalling` (`self.CharacterMovement`)) (`self.ActorHasTag` OtherActor "RunWall"))
    (bind (_direction _newtrack_0) (`Timeline|Timeline_0` :!via `PlayFromStart` :!label _label_6)
      (:`Update`
        (`Controller.SetControlRotation` (`GameplayStatics.GetPlayerController` 0) (`KismetMathLibrary.RLerp` _returnvalue (`KismetMathLibrary.MakeRotator` 20.0 (.pitch _returnvalue) (.yaw _returnvalue)) _newtrack_0))))))

(event `self.LeftDetector.OnComponentEndOverlap`
  (params (OverlappedComponent :type "PrimitiveComponent Object Reference") (OtherActor :type "Actor Object Reference") (OtherComp :type "PrimitiveComponent Object Reference") (OtherBodyIndex :type Integer))
  ;[1 1 1] WallRunningSmoothing
  (if (and (`NavMovementComponent.IsFalling` (`self.CharacterMovement`)) (`self.ActorHasTag` (stale `self.LeftDetector.OnComponentBeginOverlap` OtherActor) "RunWall"))
    (goto _label_6 :!via `ReverseFromEnd`)))

(fn `UserConstructionScript`)